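; Enemy actor Blueprint that holds health and death state and can detect the player in front of it.
; BeginPlay resets Hp to full and clears the IsEnemyDie flag; overlap, tick and construction logic are empty.
; CanSeePlayer runs a short debug-drawn forward line trace from the actor's location, returning whether the hit actor has the HERO tag, plus that actor.
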(event `self.ReceiveBeginPlay`
  (set `self.IsEnemyDie` false)
  (set `self.hp` 100.0))

(fn `CanSeePlayer`
  (returns (value :type Boolean) (player :type "Actor Object Reference"))
  (bind _returnvalue (`self.K2_GetActorLocation`))
  (bind (_outhit _returnvalue_2) (`KismetSystemLibrary.LineTraceSingle` :`Start` _returnvalue :`End` (+ _returnvalue (* (`self.GetActorForwardVector`) 500)) :`TraceChannel` "TraceTypeQuery3" :`DrawDebugType` "ForDuration"))
  (if _returnvalue_2
    (bind (_bblockinghit _binitialoverlap _time _location _impactpoint _normal _impactnormal _physmat _hitactor) (`GameplayStatics.BreakHitResult` _outhit))
    (return (`self.ActorHasTag` _hitactor "HERO") _hitactor)
    (else
      (return false null))))

(fn `UserConstructionScript`)