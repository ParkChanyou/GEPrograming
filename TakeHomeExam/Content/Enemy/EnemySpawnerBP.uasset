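; Enemy spawner that periodically spawns EnemyBP AI pawns at random points inside its Box component.
; On BeginPlay it caches the ShooterGameMode and starts a looping one-second timer.
; Each tick of the timer spawns only while the game mode's enemy count is within its cap, stamps the current count onto the new enemy as its Number, then increments the shared count.
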(event `self.ReceiveBeginPlay`
  (bind _asshooter_game_mode (cast `/Game/ShooterGameMode` (`GameplayStatics.GetGameMode`)))
  (set `self.GameMode` _asshooter_game_mode)
  (`KismetSystemLibrary.K2_SetTimer` null "SpawnEnemy" 1.0 true))

(event `SpawnEnemy`
  (bind _box (`self.Box`))
  (bind _gamemode (`self.GameMode`))
  (if (<= (`/Game/ShooterGameMode.NumberEnemy` (`self.GameMode`)) 10.0)
    (bind _returnvalue (`AIBlueprintHelperLibrary.SpawnAIFromClass` "/Game/Enemy/EnemyBP.EnemyBP_C" null (`KismetMathLibrary.RandomPointInBoundingBox` (`SceneComponent.K2_GetComponentLocation` _box) (`BoxComponent.GetScaledBoxExtent` _box))))
    (bind _asenemy_bp (cast `/Game/Enemy/EnemyBP` _returnvalue))
    (set `/Game/Enemy/EnemyBP.number` (`/Game/ShooterGameMode.NumberEnemy` _gamemode) _asenemy_bp)
    (`/Game/ShooterGameMode.IncreaseEnemy` _gamemode)))

(fn `UserConstructionScript`)