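; HeroBP is the player-controlled hero in a shooter, handling movement, firing and health.
; On BeginPlay it sets health and spawns a GunBP attached to the mesh's GunPoint socket, with the trigger input starting and stopping fire.
; Axis inputs move it along fixed world axes and yaw the actor.
; DecreaseHP reports health to ShooterGameMode and restarts the level by console command when health runs out.
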(event `self.ReceiveBeginPlay`
  (set `self.hp` 100.0)
  (bind _returnvalue (`|SpawnActorFromClass` "/Game/Gun/GunBP.GunBP_C" (`SceneComponent.K2_GetComponentToWorld` (`self.Mesh`)) "Undefined" "OverrideRootScale"))
  (bind _output_get (set `self.Gun` _returnvalue))
  (`self.K2_AttachToComponent` _output_get (`self.Mesh`) "GunPoint" "SnapToTarget" "SnapToTarget" "KeepWorld" true))

(event `InputAxis|MoveForward`
  (params (AxisValue :type "Float (single-precision)"))
  (`self.AddMovementInput` (1.0 0.0 0.0) AxisValue))

(event `InputAxis|MoveRight`
  (params (AxisValue :type "Float (single-precision)"))
  (`self.AddMovementInput` (0.0 1.0 0.0) AxisValue))

(event `InputAxis|TurnRight`
  (params (AxisValue :type "Float (single-precision)"))
  (`self.K2_AddActorWorldRotation` (`KismetMathLibrary.MakeRotator` 0.0 0.0 AxisValue)))

(event `InputAction|TriggerBullet`
  (params (Key :type "Key Structure" :default "AnyKey"))
  (bind _gun (`self.Gun`))
  (:`Pressed`
    (`/Game/Gun/GunBP.StartFire` _gun))
  (:`Released`
    (`/Game/Gun/GunBP.StopFire` _gun)))

(event `/Game/DamageInterface.DecreaseHP`
  (params (Amount :type "Float (single-precision)"))
  (bind _output_get (set `self.hp` (- (`self.hp`) Amount)))
  (bind _asshooter_game_mode (cast `/Game/ShooterGameMode` (`GameplayStatics.GetGameMode`)))
  (`/Game/ShooterGameMode.UpdateHeroHP` _asshooter_game_mode _output_get)
  (if (<= _output_get 0.0)
    (`KismetSystemLibrary.ExecuteConsoleCommand` "RestartLevel")))

(fn `UserConstructionScript`)